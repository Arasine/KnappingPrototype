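; Knapping grid actor that spawns a BP_KnappCube for each of GridSize × GridSize cells on BeginPlay.
; Cubes spawn at one-fifth scale at fixed height, using XCoord and YCoord plus a fixed world offset, independent of the actor's transform.
; XCoord wraps to a new YCoord row past the grid edge, but this graph never increments XCoord and applies no cell spacing multiplier.
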(event `self.ReceiveBeginPlay`
  (bind _gridsize (`self.GridSize`))
  (for _ (range 1 (+ (* _gridsize _gridsize) 1))
    (if (> (`self.X_Coord`) (- (`self.GridSize`) 1)) :!label _label
      (set `self.X_Coord` 0)
      (bind _result (`/Engine/EditorBlueprintResources/StandardMacros.IncrementInt` (`self.Y_Coord`))
        (:`  `
          (set `self.Y_Coord` _result)
          (goto _label)))
      (else
        (`|SpawnActorFromClass` "/Game/FirstPerson/Blueprints/BP_KnappCube.BP_KnappCube_C" (`KismetMathLibrary.MakeTransform` (`KismetMathLibrary.MakeVector` (`KismetMathLibrary.Conv_IntToDouble` (+ (`self.X_Coord`) 1000)) (`KismetMathLibrary.Conv_IntToDouble` (+ (`self.Y_Coord`) 1000)) 20.0) (struct) (0.2 0.2 0.2)) "Undefined" "MultiplyWithRoot" null null)))))

(fn `UserConstructionScript`)